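; BP_ItemSpawner is an actor that periodically spawns random falling items inside a box area.
; A looping timer started on BeginPlay picks a random entry from the MeshManager's MeshData.
; It spawns a BP_FallingItem at a random point within SpawnArea, passing that entry's mesh type, points and static mesh.
; The SpawnItem function it calls is an empty stub, so the spawn logic lives in the timer event.
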(event `self.ReceiveBeginPlay`
  (`KismetSystemLibrary.K2_SetTimerDelegate` (delegate `TimerSpawn`) (`self.SpawnInterval`) true))

(event `TimerSpawn`
  (bind _spawnarea (`self.SpawnArea`))
  (bind (_points _meshtype _staticmesh) (break `/Game/Blueprints/ST_MeshData` (`self.SelectedItem`)))
  (`self.SpawnItem`)
  (set `self.SelectedItem` (`KismetArrayLibrary.Array_Random` (`/Game/Blueprints/BP_BakedGoods.MeshData` (`self.MeshManager`))))
  (`|SpawnActorFromClass` "/Game/Blueprints/BP_FallingItem.BP_FallingItem_C" (`KismetMathLibrary.MakeTransform` (`KismetMathLibrary.RandomPointInBoundingBox` (`SceneComponent.K2_GetComponentLocation` _spawnarea) (`BoxComponent.GetScaledBoxExtent` _spawnarea))) "Undefined" "MultiplyWithRoot" null _meshtype _points null _staticmesh null))

(fn `SpawnItem`)

(fn `UserConstructionScript`)